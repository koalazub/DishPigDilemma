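; Game manager for a dishwashing game that handles dish state, the round timer, audio and a stub score.
; DishChangeEvent takes the touched object from the first Sink_Blueprint and, based on IsDirty, applies a clean or dirty material chosen by state index.
; BeginPlay initializes the state and self-reference, then starts background music; SoundEffects plays indexed clips cut off after a second.
; Tick accumulates time and shows the end-game menu once at thirty seconds.
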(event `Dish Change Event`
  ;[0.009696 0.4045 5e-06] Grabs the object being touched by SinkBP and alters its state from dirty to clean and vice versa
  (bind _outactors (`GameplayStatics.GetAllActorsOfClass` "/Game/KoalaPrint/Blueprints/Sink_Blueprint.Sink_Blueprint_C"))
  (if (`self.IsDirty`)
    (bind _touchedobject (`/Game/KoalaPrint/Blueprints/Sink_Blueprint.TouchedObject` (`KismetArrayLibrary.Array_Get` _outactors)))
    (`self.SetToClean` _touchedobject)
    (else
      (`self.SetToDirty` _touchedobject))))

(event `self.ReceiveTick`
  (params (DeltaSeconds :type "Float (single-precision)"))
  ;[0.009696 0.4045 5e-06] Timer
  (`self.Timer` DeltaSeconds))

(event `self.ReceiveBeginPlay`
  ;[0.009696 0.4045 5e-06] Dish is dirty, set instantiated object as GM Object
  (`self.IntialProcess`
    (:`Function Exec`
      (`self.BGM`))))

(event `BGM`
  ;[1 0 0.795] Event for BGM
  (`GameplayStatics.PlaySoundAtLocation` (`KismetArrayLibrary.Array_Get` (`self.ABackgroundSounds`) (`self.BGMSoundIndex`))))

(event `Sound Effects`
  ;[1 0 0.795] Sound Effects Event for pick ups, drops and stuff
  (bind _returnvalue (`GameplayStatics.SpawnSoundAtLocation` (`KismetArrayLibrary.Array_Get` (`self.ASoundEffects`) (`self.SoundEffectsIndex`))))
  (`KismetSystemLibrary.PrintString` "calling sound")
  (`KismetSystemLibrary.Delay` 1.0)
  (`AudioComponent.Stop` _returnvalue))

(fn `Score`
  (set `self.MoneyScore` 10.0))

(fn `SetToClean`
  (params (DishTarget :type "DestructibleComponent Object Reference"))
  ;[0.009696 0.4045 5e-06] Grabs object parsed by Sink and alters its state according to dirty/clean
  (set `self.DishStateIndex` 1)
  (switch `/Game/KoalaPrint/EHygieneState` "NewEnumerator0"
    (:`NewEnumerator1`
      (`KismetSystemLibrary.PrintString` "casting"))
    (:`NewEnumerator0`
      (for _ (range (`PrimitiveComponent.GetNumMaterials` DishTarget))
        (`PrimitiveComponent.SetMaterial` DishTarget 0 (`self.GetDishStateAndIndex`)))
      (`KismetSystemLibrary.PrintString` "Setting Material for DirtyFunction"))))

(fn `SetToDirty`
  (params (DishTarget :type "DestructibleComponent Object Reference"))
  ;[0.009696 0.4045 5e-06] Change the dish to dirty by getting the object and setting its primitive material to dirty
  (set `self.DishStateIndex` 0)
  (switch `/Game/KoalaPrint/EHygieneState` "NewEnumerator1"
    (:`NewEnumerator1`
      (for _ (range (`PrimitiveComponent.GetNumMaterials` DishTarget))
        (`PrimitiveComponent.SetMaterial` DishTarget 0 (`self.GetDishStateAndIndex`)))
      (`KismetSystemLibrary.PrintString` "Setting material to dirty"))))

(fn `Timer`
  (params (AddTime :type "Float (double-precision)"))
  (bind _output_get (set `self.SecondsPassed` (+ AddTime (`self.SecondsPassed`))))
  (if (>= _output_get 30.0)
    (if (not (`self.HasMenuSpawned`))
      (bind _returnvalue (`|CreateWidget` "/Game/KoalaPrint/MenuBluePrints/EndGameMenu.EndGameMenu_C"))
      (`UserWidget.AddToViewport` _returnvalue 0)
      (`WidgetBlueprintLibrary.SetInputMode_UIOnlyEx` null _returnvalue)
      (set `self.HasMenuSpawned` true))))

(fn `UserConstructionScript`)