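; DishSpawningArea is an area actor that keeps spawning random items from its SpawnableItems list inside its own bounds.
; It spawns an initial batch of five on BeginPlay, then Tick accumulates time and spawns another each time the ItemSpawnTimer interval elapses.
; SpawnItem picks a random class and places it at a random point within the box returned by GetActorArrayBounds on itself.
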(event `self.ReceiveBeginPlay`
  (`self.SpawnItem`)
  (`self.SpawnItem`)
  (`self.SpawnItem`)
  (`self.SpawnItem`)
  (`self.SpawnItem`))

(event `self.ReceiveTick`
  (params (DeltaSeconds :type "Float (single-precision)"))
  (bind _output_get (set `self.timer` (+ (`self.timer`) DeltaSeconds)))
  (if (>= _output_get (`self.ItemSpawnTimer`))
    (`self.SpawnItem`)
    (set `self.timer` 0.0)))

(fn `SpawnItem`
  (bind (_center _boxextent) (`GameplayStatics.GetActorArrayBounds` (`|MakeArray` self :!type "Actor Object Reference")))
  (`|SpawnActorFromClass` (`KismetArrayLibrary.Array_Get` (`self.spawnableItems`) (`KismetMathLibrary.RandomIntegerInRange` 0 (- (`KismetArrayLibrary.Array_Length` (`self.spawnableItems`)) 1))) (`KismetMathLibrary.MakeTransform` (`KismetMathLibrary.MakeVector` (+ (.x _center) (`KismetMathLibrary.RandomFloatInRange` (* (.x _boxextent) -1.0) (.x _boxextent))) (+ (.y _center) (`KismetMathLibrary.RandomFloatInRange` (* (.y _boxextent) -1.0) (.y _boxextent))) (+ (.z _center) (`KismetMathLibrary.RandomFloatInRange` (* (.z _boxextent) -1.0) (.z _boxextent))))) "Undefined" "OverrideRootScale"))

(fn `UserConstructionScript`)